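; Maze actor that lays out a Width by Length grid of cells and walls centered on itself.
; Construction script rebuilds instanced previews of every cell and possible wall from the size, thickness and height settings.
; HandleCellAdded attaches each new cell, moves it to its grid position and sets its size.
; Shared helpers convert cell or wall coordinates to local positions, spacing by cell width plus wall thickness and offsetting walls half a step.
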(event `self.HandleCellAdded`
  (params (NewCell :type "Cell Object Reference"))
  (bind _cellwidth (`self.CellWidth`))
  (`|ExecutionSequence`
    (:`then_0`
      (`self.K2_AttachToActor` NewCell self "None" "SnapToTarget" "SnapToTarget" "SnapToTarget" false)
      (bind _result (`self.GetPositionForCell` NewCell))
      (`self.K2_SetActorRelativeLocation` NewCell _result false true))
    (:`then_1`
      (`Cell.SetCellSize` NewCell (`KismetMathLibrary.MakeVector2D` _cellwidth _cellwidth)))))

(fn `GetCellOffset`
  (params (Column :type Integer) (Row :type Integer))
  (returns (ReturnValue :type "Vector2D Structure"))
  (return (* (- (`KismetMathLibrary.MakeVector2D` (`KismetMathLibrary.Conv_IntToDouble` Column) (`KismetMathLibrary.Conv_IntToDouble` Row)) (/ (- (`KismetMathLibrary.MakeVector2D` (`KismetMathLibrary.Conv_IntToDouble` (`self.Width`)) (`KismetMathLibrary.Conv_IntToDouble` (`self.Length`))) 1.0) 2.0)) (`self.GetCellSpacing`))))

(fn `GetCellSpacing`
  (returns (FullWidth :type "Float (double-precision)"))
  (return (+ (`self.CellWidth`) (`self.WallThickness`))))

(fn `GetPositionForCell`
  (params (Cell :type "Cell Object Reference"))
  (returns (Result :type "Vector Structure"))
  (bind (_returnvalue_maze _returnvalue_cellcolumn _returnvalue_cellrow) (break `CellCoordinates` (`self.GetCellCoordinates` Cell)))
  (bind _result (`self.GetPositionForCellCoordinates` _returnvalue_cellcolumn _returnvalue_cellrow))
  (return _result))

(fn `GetPositionForCellCoordinates`
  (params (Column :type Integer) (Row :type Integer))
  (returns (Result :type "Vector Structure"))
  (bind _returnvalue (`self.GetCellOffset` Column Row))
  (return (`KismetMathLibrary.Conv_Vector2DToVector` _returnvalue)))

(fn `GetPositionForWall`
  (params (Wall :type "Wall Object Reference"))
  (returns (Result :type "Vector Structure"))
  (bind (_returnvalue_maze _returnvalue_wallcolumn _returnvalue_wallrow _returnvalue_walldirection) (break `WallCoordinates` (`self.GetWallCoordinates` Wall)))
  (bind _result (`self.GetPositionForWallCoordinates` _returnvalue_wallcolumn _returnvalue_wallrow _returnvalue_walldirection))
  (return _result))

(fn `GetPositionForWallCoordinates`
  (params (Column :type Integer) (Row :type Integer) (WallDirection :type "EWallDirection Enum" :default "EWD_NS"))
  (returns (Result :type "Vector Structure"))
  (bind _returnvalue (`self.GetWallOffset` Column Row WallDirection))
  (return (`KismetMathLibrary.Conv_Vector2DToVector` _returnvalue)))

(fn `GetWallOffset`
  (params (Column :type Integer) (Row :type Integer) (WallDirection :type "EWallDirection Enum" :default "EWD_NS"))
  (returns (ReturnValue :type "Vector2D Structure"))
  (bind _returnvalue (/ (`self.GetCellSpacing`) -2.0))
  (bind _returnvalue_2 (`self.GetCellOffset` Column Row))
  (return (+ _returnvalue_2 (select `EWallDirection` WallDirection :`EWD_NS` (`KismetMathLibrary.MakeVector2D` 0.0 _returnvalue) :`EWD_WE` (`KismetMathLibrary.MakeVector2D` _returnvalue)))))

(fn `UserConstructionScript`
  (bind _returnvalue (/ (`self.CellWidth`) 100.0))
  (bind _returnvalue_2 (`KismetMathLibrary.MakeVector` 0.0 0.0 (/ (`self.WallHeight`) 2.0)))
  (`|ExecutionSequence`
    (:`then_0`
      (`InstancedStaticMeshComponent.ClearInstances` (`self.CellsPreview`))
      (bind (_row _column) (`/Game/MacroUtilsBP.ForLoop2D` 0 (- (`self.Length`) 1) 0 (- (`self.Width`) 1))
        (:`LoopBody`
          (bind _result (`self.GetPositionForCellCoordinates` _column _row))
          (`InstancedStaticMeshComponent.AddInstance` (`self.CellsPreview`) (`KismetMathLibrary.MakeTransform` _result (struct) (`KismetMathLibrary.MakeVector` _returnvalue _returnvalue 0.1))))))
    (:`then_1`
      (`InstancedStaticMeshComponent.ClearInstances` (`self.WallsPreview`))
      (`|ExecutionSequence`
        (:`then_0`
          (bind (_row_2 _column_2) (`/Game/MacroUtilsBP.ForLoop2D` 0 (- (`self.Length`) 1) 0 (`self.Width`))
            (:`LoopBody`
              (bind _result_2 (`self.GetPositionForWallCoordinates` _column_2 _row_2 "EWD_WE"))
              (`InstancedStaticMeshComponent.AddInstance` (`self.WallsPreview`) (`KismetMathLibrary.MakeTransform` (+ _result_2 _returnvalue_2) (struct) (/ (`KismetMathLibrary.MakeVector` (`self.WallThickness`) (`self.GetCellSpacing`) (`self.WallHeight`)) 100.0))))))
        (:`then_1`
          (bind (_row_3 _column_3) (`/Game/MacroUtilsBP.ForLoop2D` 0 (`self.Length`) 0 (- (`self.Width`) 1))
            (:`LoopBody`
              (bind _result_3 (`self.GetPositionForWallCoordinates` _column_3 _row_3))
              (`InstancedStaticMeshComponent.AddInstance` (`self.WallsPreview`) (`KismetMathLibrary.MakeTransform` (+ _result_3 _returnvalue_2) (struct) (/ (`KismetMathLibrary.MakeVector` (`self.GetCellSpacing`) (`self.WallThickness`) (`self.WallHeight`)) 100.0))))))))))