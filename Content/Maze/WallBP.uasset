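; Maze wall Blueprint that exposes events for sizing a wall piece by height, thickness and width.
; Each event rescales one axis of VisualRoot and keeps the other two: height on Z, thickness on X and width on Y.
; Inputs are converted to scale factors by fixed divisors, with thickness using a different one from height and width.
; The facing-direction event is an empty stub, and the construction script does nothing.
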(event `self.SetWallHeight`
  (params (NewHeight :type "Float (single-precision)"))
  (bind _visualroot (`self.VisualRoot`))
  (`SceneComponent.SetRelativeScale3D` _visualroot (`KismetMathLibrary.MakeVector` (.x (`SceneComponent.RelativeScale3D` _visualroot)) (.y (`SceneComponent.RelativeScale3D` _visualroot)) (/ NewHeight 100.0))))

(event `self.SetWallThickness`
  (params (NewThickness :type "Float (single-precision)"))
  (bind _visualroot (`self.VisualRoot`))
  (`SceneComponent.SetRelativeScale3D` _visualroot (`KismetMathLibrary.MakeVector` (/ NewThickness 10.0) (.y (`SceneComponent.RelativeScale3D` _visualroot)) (.z (`SceneComponent.RelativeScale3D` _visualroot)))))

(event `self.SetWallWidth`
  (params (NewWidth :type "Float (single-precision)"))
  (bind _visualroot (`self.VisualRoot`))
  (`SceneComponent.SetRelativeScale3D` _visualroot (`KismetMathLibrary.MakeVector` (.x (`SceneComponent.RelativeScale3D` _visualroot)) (/ NewWidth 100.0) (.z (`SceneComponent.RelativeScale3D` _visualroot)))))

(event `self.SetWallFacingDirection`
  (params (NewFacingDir :type "Vector Structure (by ref)")))

(fn `UserConstructionScript`)